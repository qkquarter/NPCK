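; BP_InterFace holds combat hit logic that turns an attack into HP, posture and knockback results.
; AttackEvent passes damage and posture through a collapsed graph to GetCurrentHP and GetCurrentPosture, returning their results.
; Knockback is the normalized attacker location scaled by negative impact, with no victim position subtracted.
; Both getter graphs contain only unconnected subtraction nodes.
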(fn AttackEvent
  (params (Damage :type Float%20%28double-precision%29) (Posture :type Float%20%28double-precision%29) (Imfact :type Float%20%28double-precision%29) (AttackerLoc :type Vector))
  (bind (_hp _stamina) (|CollapseGraph Damage Posture))
  (return _hp _stamina (* (* Imfact -1.0) (Math|Vector|Normalize AttackerLoc))))